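; Enemy character Blueprint that roams at random and chases actors tagged Hero that enter its PlayerDetection component.
; Roaming picks a nearby navigable point, spawns an AI_Destination actor there and calls AIMoveTo, repeating on success or failure.
; A Hero overlap stores the target and moves toward it.
; The Hero leaving, or any non-Hero overlap, clears the target and restarts roaming.
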(event OnComponentBeginOverlap(PlayerDetection)
  (params (OverlappedComponent :type Primitive%20Component%20Object%20Reference) (OtherActor :type Actor%20Object%20Reference) (OtherComp :type Primitive%20Component%20Object%20Reference) (OtherBodyIndex :type Integer) (bFromSweep :type Boolean) (SweepResult :type Hit%20Result%20Structure%20%28by%20ref%29))
  (if (Actor|ActorHasTag OtherActor "Hero")
    (Variables|Default|SetOther%20Actor OtherActor)
    (CallFunction|Chase)
    (else
      (Variables|Default|SetOther%20Actor 0)
      (CallFunction|Roaming))))

(event OnComponentEndOverlap(PlayerDetection)
  (params (OverlappedComponent :type Primitive%20Component%20Object%20Reference) (OtherActor :type Actor%20Object%20Reference) (OtherComp :type Primitive%20Component%20Object%20Reference) (OtherBodyIndex :type Integer))
  (if (Actor|ActorHasTag OtherActor "Hero")
    (Variables|Default|SetOther%20Actor 0)
    (CallFunction|Roaming)))

(event Custom|Roaming
  (bind _randomlocation (Class|NavigationSystemV1|GetRandomLocationinNavigableRadius (Transformation|GetActorLocation) 5e+02 0 0))
  (Game|SpawnActorfromClass "/Game/ProceduralLevel/Characters/Enemies/AI_Destination.AI_Destination_C" (Math|Transform|MakeTransform _randomlocation "0, 0, 0" "1.000000,1.000000,1.000000") "AlwaysSpawn" "MultiplyWithRoot" 0 0)
  (AI|AIMoveTo self _randomlocation (Variables|Default|GetOther%20Actor) 5.0 false
    (:OnSuccess
      _)
    (:OnFail
      _))
  (CallFunction|Roaming))

(event Custom|chase
  (AI|AIMoveTo self "0, 0, 0" (Variables|Default|GetOther%20Actor) 5.0 false))

(event EventBeginPlay
  (CallFunction|Roaming))

(fn ConstructionScript)